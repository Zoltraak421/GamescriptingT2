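; Base enemy actor that takes damage when a BP_Projectile overlaps it.
; Overlap subtracts the projectile's Damage from Health through the Applydamage event.
; At zero health it plays a death sound, triggers camera shake on myPlayerController and destroys itself.
; Otherwise it plays a hit sound and briefly flashes every static mesh component with a damage overlay material, cleared after a short delay.
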(event `self.ReceiveActorBeginOverlap`
  (params (OtherActor :type "Actor Object Reference"))
  (bind _asbp_projectile (cast `/Game/Blueprints/BP_Projectile` OtherActor))
  (`self.Applydamage` (`/Game/Blueprints/BP_Projectile.Damage` _asbp_projectile))
  ; checks if health is depleated
  (if (<= (`self.health`) 0.0)
    (`GameplayStatics.PlaySound2D` "/Game/Sci-Fi_Shots_Pack2_Game_Of_Weapons/Wave/SciFi_Shot_P2__110_.SciFi_Shot_P2__110_" 1.0 1.0 0.0 null null)
    (`|ExecutionSequence`
      (:`then_0`
        (bind _asmy_player_controller (cast `/Game/Framework/myPlayerController` (`GameplayStatics.GetPlayerController` 0)))
        (`/Game/Framework/myPlayerController.Apply Camera Shake` _asmy_player_controller))
      (:`then_1`
        (`self.K2_DestroyActor`)))
    (else
      (`GameplayStatics.PlaySound2D` "/Game/Sci-Fi_Shots_Pack2_Game_Of_Weapons/Wave/SciFi_Shot_P2__105_.SciFi_Shot_P2__105_" 1.0 1.0 0.0 null null)
      (for _array_element (`self.K2_GetComponentsByClass` "/Script/Engine.StaticMeshComponent")
        (`MeshComponent.SetOverlayMaterial` _array_element "/Game/Materials/MI_Damage_flash.MI_Damage_flash"))
      (`KismetSystemLibrary.Delay` 0.2)
      (for _array_element_2 (`self.K2_GetComponentsByClass` "/Script/Engine.StaticMeshComponent")
        (`MeshComponent.SetOverlayMaterial` _array_element_2 null))
      (`KismetSystemLibrary.Delay` 0.2))))

(event `Applydamage`
  (params (Damage :type "Float (double-precision)"))
  ; does damage
  (set `self.health` (- (`self.health`) Damage)))

(fn `UserConstructionScript`)