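; Enemy spawner that repeatedly spawns random enemies from a class pool, each facing a random target point.
; BeginPlay starts a looping timer whose 1–5 second interval is rolled once, so the spawn rate stays fixed afterwards.
; Each spawn picks random locations on the StartPoint and EndPoint splines, placing the enemy on the first and rotating it toward the second.
; All random picks draw from a shared RandomStream.
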(event `self.ReceiveTick`
  (params (DeltaSeconds :type "Float (single-precision)")))

(event `self.ReceiveBeginPlay`
  ; Enemy Spawner
  (bind _returnvalue (`KismetSystemLibrary.K2_SetTimerDelegate` (delegate `SpawnEnemy`) (`KismetMathLibrary.RandomFloatInRangeFromStream` (`self.randomStream`) 1.0 5.0) true true))
  (set `self.EnemySpawnTimer` _returnvalue))

(event `SpawnEnemy`
  ; Enemy Spawner
  (bind (_newparam _newparam1) (`self.StartAndEndPoint`))
  (`|SpawnActorFromClass` (`KismetArrayLibrary.Array_RandomFromStream` (`self.EnemyClassPool`) (`self.randomStream`)) (`KismetMathLibrary.MakeTransform` _newparam (`KismetMathLibrary.FindLookAtRotation` _newparam _newparam1)) "Undefined" "MultiplyWithRoot" null null))

(fn `StartAndEndPoint`
  (returns (NewParam :type "Vector Structure") (NewParam1 :type "Vector Structure"))
  (bind _returnvalue (`KismetMathLibrary.RandomFloatFromStream` (`self.randomStream`)))
  (return (`SplineComponent.GetLocationAtTime` (`self.StartPoint`) _returnvalue "World" false) (`SplineComponent.GetLocationAtTime` (`self.EndPoint`) _returnvalue "World" false)))

(fn `UserConstructionScript`)